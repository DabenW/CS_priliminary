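; First-person player character Blueprint with movement, look, jump, sprint and automatic hitscan rifle fire.
; Movement follows control rotation, and sprint adds and subtracts a speed offset on the current max walk speed.
; Holding fire plays a montage and muzzle flash while a looping timer calls ShootOnce until release.
; ShootOnce line-traces from the camera along the view direction and damages any TppCharacter hit.
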(event `InputAxis|moveForward`
  (params (AxisValue :type "Float (single-precision)"))
  (`self.AddMovementInput` (`KismetMathLibrary.GetForwardVector` (`self.GetControlRotation`)) AxisValue))

(event `InputAxis|moveLeft`
  (params (AxisValue :type "Float (single-precision)"))
  (`self.AddMovementInput` (`KismetMathLibrary.GetForwardVector` (`KismetMathLibrary.ComposeRotators` (`self.GetControlRotation`) (`KismetMathLibrary.MakeRotator` 0.0 0.0 -90.0))) AxisValue))

(event `InputAxis|turn`
  (params (AxisValue :type "Float (single-precision)"))
  (`self.AddControllerYawInput` AxisValue))

(event `InputAxis|up`
  (params (AxisValue :type "Float (single-precision)"))
  (`self.AddControllerPitchInput` AxisValue))

(event `InputAction|jump`
  (params (Key :type "Key Structure" :default "AnyKey"))
  (:`Pressed`
    (`self.Jump`)))

(event `InputAction|fire`
  (params (Key :type "Key Structure" :default "AnyKey"))
  (:`Pressed`
    (`self.startFire`) ; 包含了对集中的判定
  )
  (:`Released`
    (`self.endFire`) ; 包含了对击打的取消
  ))

(event `InputAction|fastMove`
  (params (Key :type "Key Structure" :default "AnyKey"))
  (bind _charactermovement (`self.CharacterMovement`))
  (bind _addspeed (`self.addSpeed`))
  (bind _returnvalue (`MovementComponent.GetMaxSpeed` _charactermovement))
  (:`Pressed`
    (set `CharacterMovementComponent.MaxWalkSpeed` (+ _returnvalue _addspeed) _charactermovement))
  (:`Released`
    (set `CharacterMovementComponent.MaxWalkSpeed` (- _returnvalue _addspeed) _charactermovement)))

(fn `endFire`
  (`|ExecutionSequence`
    (:`then_0`
      (`self.StopAnimMontage` "/Game/Blueprints/FppCharacter_Montage.FppCharacter_Montage")
      (`ActorComponent.K2_DestroyComponent` (`self.FireEffect`)))
    (:`then_1`
      (`KismetSystemLibrary.K2_ClearTimer` null "shootonce"))))

(fn `shootOnce`
  (bind _returnvalue (`SceneComponent.K2_GetComponentLocation` (`self.Camera`)))
  (bind (_outhit _returnvalue_2) (`KismetSystemLibrary.LineTraceSingle` _returnvalue (+ (* (`KismetMathLibrary.Normal` (`KismetMathLibrary.GetForwardVector` (`self.GetControlRotation`))) 1500.0) _returnvalue) "TraceTypeQuery1"))
  (if _returnvalue_2
    (bind _astpp_character (cast `/Game/Blueprints/TppCharacter` (`.HitActor` (`GameplayStatics.BreakHitResult` _outhit)))) ; 类型转换
    (`/Game/Blueprints/TppCharacter.takeDamage` _astpp_character 20.0)))

(fn `startFire`
  (`|ExecutionSequence`
    (:`then_0`
      (`self.PlayAnimMontage` "/Game/Blueprints/FppCharacter_Montage.FppCharacter_Montage")
      (bind _returnvalue (`GameplayStatics.SpawnEmitterAttached` "/Game/Assets/Effects/ParticleSystems/Weapons/AssaultRifle/Muzzle/P_AssaultRifle_MF.P_AssaultRifle_MF" (`self.fireEffectArrow`)))
      (set `self.FireEffect` _returnvalue))
    (:`then_1`
      (`self.shootOnce`)
      (`KismetSystemLibrary.K2_SetTimer` null "shootOnce" 0.2 true))))

(fn `UserConstructionScript`)