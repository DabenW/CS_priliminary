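; A third-person character Blueprint that tracks health and dies when it runs out.
; The construction script sets the mesh to block the Visibility channel, so line traces on that channel can hit it.
; TakeDamage subtracts from Health and prints the new value.
; When IsDead is true, it detaches the controller and starts a short named timer for OnDieOver, which destroys the actor.
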(fn `isDead`
  (returns (isDead :type Boolean))
  (return (<= (`self.health`) 0.0)))

(fn `onDieOver`
  (`self.K2_DestroyActor`))

(fn `takeDamage`
  (params (damage :type "Float (double-precision)"))
  (bind _output_get (set `self.health` (- (`self.health`) damage)))
  (`KismetSystemLibrary.PrintString` (`KismetStringLibrary.Conv_DoubleToString` _output_get))
  (if (`self.isDead`)
    (`self.DetachFromControllerPendingDestroy`)
    (`KismetSystemLibrary.K2_SetTimer` null "onDieOver" 2.0)))

(fn `UserConstructionScript`
  (`PrimitiveComponent.SetCollisionResponseToChannel` (`self.Mesh`) "ECC_Visibility" "ECR_Block"))